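; Track switch actor for trains, with a straight spline and left and right curves, starting on the right curve.
; Construction snaps spline ends to nearby BP_Track spline points, samples each spline into waypoint arrays and moves three trigger boxes to the junction endpoints.
; An overlapping train pawn's entrance side and direction, inverted in gear index zero, feed CalculateValidSpline, whose body is not shown.
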(event `self.LeftBox.OnComponentBeginOverlap`
  (params (OverlappedComponent :type "PrimitiveComponent Object Reference") (OtherActor :type "Actor Object Reference") (OtherComp :type "PrimitiveComponent Object Reference") (OtherBodyIndex :type Integer) (bFromSweep :type Boolean) (SweepResult :type "HitResult Structure (by ref)"))
  (bind _entrance (`self.Entrance`))
  (`KismetSystemLibrary.PrintString` "Hello")
  (set `self.PlayerRef` OtherActor)
  (set `self.Entrance` "LEFT")
  (bind _asbp_train_pawn (cast `/Game/Blueprints/Player/BP_TrainPawn` (`self.PlayerRef`) :!label _label))
  (if (== (`TrainPawn.GearIndex` _asbp_train_pawn) 0)
    (bind _playerdirection (`TrainPawn.PlayerDirection` _asbp_train_pawn))
    (bind _inverseddirection (`self.InverseTrainDirection` _playerdirection))
    (`self.CalculateValidSpline` _entrance _inverseddirection)
    (else
      (`self.CalculateValidSpline` _entrance _playerdirection))))

(event `self.RightBox.OnComponentBeginOverlap`
  (params (OverlappedComponent :type "PrimitiveComponent Object Reference") (OtherActor :type "Actor Object Reference") (OtherComp :type "PrimitiveComponent Object Reference") (OtherBodyIndex :type Integer) (bFromSweep :type Boolean) (SweepResult :type "HitResult Structure (by ref)"))
  (`KismetSystemLibrary.PrintString` "Hello")
  (set `self.PlayerRef` OtherActor)
  (set `self.Entrance` "RIGHT")
  (goto _label))

(event `self.FrontBox.OnComponentBeginOverlap`
  (params (OverlappedComponent :type "PrimitiveComponent Object Reference") (OtherActor :type "Actor Object Reference") (OtherComp :type "PrimitiveComponent Object Reference") (OtherBodyIndex :type Integer) (bFromSweep :type Boolean) (SweepResult :type "HitResult Structure (by ref)"))
  (`KismetSystemLibrary.PrintString` "Hello")
  (set `self.PlayerRef` OtherActor)
  (set `self.Entrance` "CENTER")
  (goto _label))

(event `self.ReceiveBeginPlay`
  (set `self.ActiveSpline` (`self.CurveToRight`)))

(fn `GetClosestSplinePoint`
  (params (SplineComponent :type "SplineComponent Object Reference") (Point :type "Vector Structure"))
  (returns (PointIndex :type Integer))
  (locals (MinimalDistance :type "Float (double-precision)" :default 99999.0) (MinimalPoint :type Integer))
  (for _index (range (+ (`SplineComponent.GetNumberOfSplinePoints` SplineComponent) 1))
    (bind _returnvalue (`KismetMathLibrary.Abs` (`KismetMathLibrary.Vector_Distance` Point (`SplineComponent.GetLocationAtSplinePoint` SplineComponent _index "World"))))
    (if (< _returnvalue (`local.MinimalDistance`))
      (set `local.MinimalDistance` _returnvalue)
      (set `local.MinimalPoint` _index)))
  (return (`local.MinimalPoint`)))

(fn `InverseTrainDirection`
  (params (Direction :type Integer))
  (returns (InversedDirection :type Integer))
  (if (== Direction 0)
    (return 1)
    (else
      (return 0))))

(fn `MoveCollidersToEndpoints`
  (bind _linearspline (`self.LinearSpline`))
  (`SceneComponent.K2_SetWorldLocation` (`self.LeftBox`) (`SplineComponent.GetLocationAtSplinePoint` _linearspline 0 "World") false false)
  (`SceneComponent.K2_SetWorldLocation` (`self.RightBox`) (`SplineComponent.GetLocationAtSplinePoint` _linearspline 1 "World") false false)
  (`SceneComponent.K2_SetWorldLocation` (`self.FrontBox`) (`SplineComponent.GetLocationAtSplinePoint` (`self.CurveToLeft`) 1 "World") false false))

(fn `SnapToNearest`
  (params (IndexToSnap :type Integer) (SplineRef :type "SplineComponent Object Reference"))
  (bind _returnvalue (`SplineComponent.GetLocationAtSplinePoint` SplineRef IndexToSnap "World"))
  (bind _outactors (`GameplayStatics.GetAllActorsOfClass` "/Game/Blueprints/Tracks/BP_Track.BP_Track_C"))
  (bind _returnvalue_2 (`self.GetComponentByClass` (`.ReturnValue` (`GameplayStatics.FindNearestActor` _returnvalue _outactors)) "/Script/Engine.SplineComponent"))
  (bind _pointindex (`self.GetClosestSplinePoint` _returnvalue_2 _returnvalue))
  (bind _returnvalue_3 (`SplineComponent.GetLocationAtSplinePoint` _returnvalue_2 _pointindex "World"))
  (if (<= (`KismetMathLibrary.Vector_Distance` _returnvalue _returnvalue_3) 150.0)
    (`SplineComponent.SetLocationAtSplinePoint` SplineRef IndexToSnap _returnvalue_3 "World" true)))

(fn `UserConstructionScript`
  (for (_array_element _array_index) (`|MakeArray` (`self.LinearSpline`) (`self.CurveToRight`) (`self.CurveToLeft`))
    (`self.SnapToNearest` 0 _array_element)
    (`self.SnapToNearest` 1 _array_element)
    (set `self.Distance Used` 0.0)
    (while (< (`self.Distance Used`) (`SplineComponent.GetSplineLength` _array_element))
      (switch `int` _array_index
        (:`0`
          (bind _returnvalue (`SplineComponent.GetLocationAtDistanceAlongSpline` _array_element (`self.Distance Used`) "World"))
          (`KismetArrayLibrary.Array_Add` (`self.WaypointsLinear`) _returnvalue)
          (set `self.Distance Used` (+ (`self.Distance Used`) 50.0)))
        (:`1`
          (`KismetArrayLibrary.Array_Add` (`self.WaypointsRight`) _returnvalue)
          (set `self.Distance Used` (+ (`self.Distance Used`) 50.0)))
        (:`2`
          (`KismetArrayLibrary.Array_Add` (`self.WaypointsLeft`) _returnvalue)
          (set `self.Distance Used` (+ (`self.Distance Used`) 50.0))))))
  (`self.MoveCollidersToEndpoints`))