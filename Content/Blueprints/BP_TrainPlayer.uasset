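; BP_TrainPlayer is the player's train Blueprint, handling the switch to a new track when one of its detectors overlaps a BP_Track.
; GearIndex selects the active detector: BackDetector responds at index zero, FrontDetector at any other.
; Each passes the overlapped track and a backwards flag to SwitchToNewTrack, then prints a Spanish debug message naming the trigger.
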(event `self.BackDetector.OnComponentBeginOverlap`
  (params (OverlappedComponent :type "PrimitiveComponent Object Reference") (OtherActor :type "Actor Object Reference") (OtherComp :type "PrimitiveComponent Object Reference") (OtherBodyIndex :type Integer) (bFromSweep :type Boolean) (SweepResult :type "HitResult Structure (by ref)"))
  ;[1 1 1] Atrás
  (bind _asbp_track (cast `/Game/Blueprints/BP_Track` OtherActor))
  (if (== (`self.GearIndex`) 0)
    (`self.SwitchToNewTrack` _asbp_track true)
    (`KismetSystemLibrary.PrintString` "Activador Trasero")))

(event `self.FrontDetector.OnComponentBeginOverlap`
  (params (OverlappedComponent :type "PrimitiveComponent Object Reference") (OtherActor :type "Actor Object Reference") (OtherComp :type "PrimitiveComponent Object Reference") (OtherBodyIndex :type Integer) (bFromSweep :type Boolean) (SweepResult :type "HitResult Structure (by ref)"))
  ;[1 1 1] Frente
  (bind _asbp_track (cast `/Game/Blueprints/BP_Track` OtherActor))
  (if (!= (`self.GearIndex`) 0)
    (`self.SwitchToNewTrack` _asbp_track)
    (`KismetSystemLibrary.PrintString` "Activador Delantero")))

(fn `UserConstructionScript`)