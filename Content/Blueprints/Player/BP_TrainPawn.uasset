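; BP_TrainPawn is the player train pawn, which builds a chain of trailing wagons when play begins.
; It spawns the configured number of BP_Wagon actors, each at the WagonAttach-tagged child actor component of the previous vehicle, starting from itself.
; Each wagon stores its predecessor in NextWagon, forming a linked chain.
; Possession and mesh overlaps only print debug text, and Tick draws a debug sphere at the pawn's attach point.
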(event `self.ReceivePossessed`
  (params (NewController :type "Controller Object Reference"))
  (`KismetSystemLibrary.PrintString` "POSSESSED"))

(event `self.ReceiveBeginPlay`
  (bind (_returnvalue_location _returnvalue_rotation) (`KismetMathLibrary.BreakTransform` (`SceneComponent.K2_GetComponentToWorld` (`|GetArrayItem` (`self.GetComponentsByTag` (`self.LastWagon`) "/Script/Engine.ChildActorComponent" "WagonAttach")))))
  (set `self.LastWagon` self)
  (for _ (range 1 (+ (`self.Wagons`) 1))
    (bind _returnvalue (`|SpawnActorFromClass` "/Game/Blueprints/Player/BP_Wagon.BP_Wagon_C" (`KismetMathLibrary.MakeTransform` _returnvalue_location _returnvalue_rotation) "Undefined" "OverrideRootScale" null null))
    (set `Wagon.NextWagon` (`self.LastWagon`) _returnvalue)
    (set `self.LastWagon` _returnvalue)))

(event `self.ReceiveTick`
  (params (DeltaSeconds :type "Float (single-precision)"))
  (`KismetSystemLibrary.DrawDebugSphere` (`SceneComponent.K2_GetComponentLocation` (`self.WagonAttach`)) 100.0 12 (struct :`R` 1.0 :`G` 0.811744 :`A` 1.0) 0.0 5.0))

(event `self.StaticMesh.OnComponentBeginOverlap`
  (params (OverlappedComponent :type "PrimitiveComponent Object Reference") (OtherActor :type "Actor Object Reference") (OtherComp :type "PrimitiveComponent Object Reference") (OtherBodyIndex :type Integer) (bFromSweep :type Boolean) (SweepResult :type "HitResult Structure (by ref)"))
  (`KismetSystemLibrary.PrintString` (`KismetSystemLibrary.GetDisplayName` OtherActor) true true (struct :`R` 0.543773 :`B` 1.0 :`A` 1.0)))

(fn `UserConstructionScript`)