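; BP_StationContent is a station content Blueprint that handles player spawning and station UI display.
; SpawnPlayer spawns a BP_TrainPawn at the Spawn component's world transform and has the first player controller possess it.
; DisplayStationUI creates a widget of the supplied class, stores the supplied station on the level's BP_PlayerManager, then adds the widget to the viewport.
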(event `SpawnPlayer`
  (bind _returnvalue (`|SpawnActorFromClass` "/Game/Blueprints/Player/BP_TrainPawn.BP_TrainPawn_C" (`SceneComponent.K2_GetComponentToWorld` (`self.Spawn`)) "Undefined" "OverrideRootScale" null null))
  (`KismetSystemLibrary.PrintString` "Spawned")
  (`Controller.Possess` (`GameplayStatics.GetPlayerController` 0) _returnvalue))

(event `self.ReceiveBeginPlay`)

(event `DisplayStationUI`
  (params (WdigetClass :type "UserWidget Class Reference") (Station :type "Station Object Reference"))
  (bind _returnvalue (`|CreateWidget` WdigetClass))
  (bind _returnvalue_2 (`GameplayStatics.GetActorOfClass` "/Game/Blueprints/Managers/BP_PlayerManager.BP_PlayerManager_C"))
  (set `/Game/Blueprints/Managers/BP_PlayerManager.Station` Station _returnvalue_2)
  (`UserWidget.AddToViewport` _returnvalue 0))

(fn `UserConstructionScript`)