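; BP_FuelStation is a train fuel station that shows its station UI when a train stops and can act as the player spawn point.
; It delegates both jobs to the BP_StationContent in its Station child actor.
; On train stop it logs a debug message and passes its widget class and itself to DisplayStationUI.
; At BeginPlay it calls SpawnPlayer if IsSpawnPoint is set.
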(event `self.OnTrainStopped`
  (`KismetSystemLibrary.PrintString` "Tren estacionado en fuel statio")
  (bind _asbp_station_content (cast `/Game/Blueprints/Stations/BP_StationContent` (`ChildActorComponent.ChildActor` (`self.Station`))))
  (`/Game/Blueprints/Stations/BP_StationContent.DisplayStationUI` _asbp_station_content (`self.StationWidget`) self))

(event `self.ReceiveBeginPlay`
  (if (`self.IsSpawnPoint`)
    (bind _asbp_station_content (cast `/Game/Blueprints/Stations/BP_StationContent` (`ChildActorComponent.ChildActor` (`self.Station`))))
    (`/Game/Blueprints/Stations/BP_StationContent.SpawnPlayer` _asbp_station_content)))

(fn `UserConstructionScript`)