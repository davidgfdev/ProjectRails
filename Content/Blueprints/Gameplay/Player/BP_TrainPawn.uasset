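; BP_TrainPawn is the player's train pawn, which builds its chain of trailing wagons when play begins.
; It reads the obtained wagon count from BP_PlayerManager and spawns that many BP_Wagon actors.
; Each spawns at the "WagonAttach"-tagged child actor component of the previous vehicle, starting with the train itself.
; Each new wagon's NextWagon references the vehicle ahead, forming a linked chain.
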(event `self.ReceivePossessed`
  (params (NewController :type "Controller Object Reference"))
  (`KismetSystemLibrary.PrintString` "POSSESSED"))

(event `self.ReceiveBeginPlay`
  (bind (_returnvalue_location _returnvalue_rotation) (`KismetMathLibrary.BreakTransform` (`SceneComponent.K2_GetComponentToWorld` (`|GetArrayItem` (`self.GetComponentsByTag` (`self.LastWagon`) "/Script/Engine.ChildActorComponent" "WagonAttach")))))
  (set `self.LastWagon` self)
  (bind _returnvalue (`GameplayStatics.GetActorOfClass` "/Game/Blueprints/Gameplay/Managers/BP_PlayerManager.BP_PlayerManager_C"))
  (bind _returnvalue_2 (`PlayerManager.GetWagonsObtained` _returnvalue))
  (for _ (range 1 (+ _returnvalue_2 1))
    (bind _returnvalue_3 (`|SpawnActorFromClass` "/Game/Blueprints/Gameplay/Player/BP_Wagon.BP_Wagon_C" (`KismetMathLibrary.MakeTransform` _returnvalue_location _returnvalue_rotation) "Undefined" "OverrideRootScale" null null))
    (set `Wagon.NextWagon` (`self.LastWagon`) _returnvalue_3)
    (set `self.LastWagon` _returnvalue_3)))

(fn `UserConstructionScript`)