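; BP_Track is a spline-based track segment that auto-connects to neighboring tracks and stores waypoints along its length.
; On construction, Snap moves each endpoint onto the closest spline point of the nearest other BP_Track actor if within a small threshold.
; It then places the front and back colliders at the spline ends.
; Finally, the construction script samples world-space waypoints at fixed distance intervals along the spline.
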(fn `GetClosestSplinePoint`
  (params (SplineComponent :type "SplineComponent Object Reference") (Point :type "Vector Structure"))
  (returns (PointIndex :type Integer))
  (locals (MinimalDistance :type "Float (double-precision)" :default 9999.0) (MinimalPoint :type Integer))
  (for _index (range (+ (`SplineComponent.GetNumberOfSplinePoints` SplineComponent) 1))
    (bind _returnvalue (`KismetMathLibrary.Vector_Distance` Point (`SplineComponent.GetLocationAtSplinePoint` SplineComponent _index "World")))
    (if (< _returnvalue (`local.MinimalDistance`))
      (set `local.MinimalDistance` _returnvalue)
      (set `local.MinimalPoint` _index)))
  (return (`local.MinimalPoint`)))

(fn `SnapToNearest`
  (params (IndexToSnap :type Integer))
  (bind _returnvalue (`SplineComponent.GetLocationAtSplinePoint` (`self.Spline`) IndexToSnap "World"))
  (bind _outactors (`GameplayStatics.GetAllActorsOfClass` "BP_Track_C"))
  (`KismetArrayLibrary.Array_RemoveItem` _outactors self)
  (bind _returnvalue_2 (`self.GetComponentByClass` (`.ReturnValue` (`GameplayStatics.FindNearestActor` _returnvalue _outactors)) "/Script/Engine.SplineComponent"))
  (bind _pointindex (`self.GetClosestSplinePoint` _returnvalue_2 _returnvalue))
  (bind _returnvalue_3 (`SplineComponent.GetLocationAtSplinePoint` _returnvalue_2 _pointindex "World"))
  (if (<= (`KismetMathLibrary.Vector_Distance` _returnvalue _returnvalue_3) 150.0)
    (`SplineComponent.SetLocationAtSplinePoint` (`self.Spline`) IndexToSnap _returnvalue_3 "World" true)))

(fn `UserConstructionScript`
  (locals (DistanceUsed :type "Float (double-precision)"))
  (bind _spline (`self.Spline`))
  (`self.SnapToNearest` (- (`SplineComponent.GetNumberOfSplinePoints` (`self.Spline`)) 1))
  (`self.SnapToNearest` 0)
  (`SceneComponent.K2_SetWorldLocation` (`self.FrontCollider`) (`SplineComponent.GetLocationAtSplinePoint` _spline (- (`SplineComponent.GetNumberOfSplinePoints` _spline) 1) "World") false false)
  (`SceneComponent.K2_SetWorldLocation` (`self.BackCollider`) (`SplineComponent.GetLocationAtSplinePoint` _spline 0 "World") false false)
  (while (< (`local.DistanceUsed`) (`SplineComponent.GetSplineLength` (`self.Spline`)))
    (`KismetArrayLibrary.Array_Add` (`self.Waypoints`) (`SplineComponent.GetLocationAtDistanceAlongSpline` (`self.Spline`) (`local.DistanceUsed`) "World"))
    (set `local.DistanceUsed` (+ (`local.DistanceUsed`) 50.0))))