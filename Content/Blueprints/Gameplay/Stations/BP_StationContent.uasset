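; Station content actor that can spawn the player's train pawn and display a station UI.
; SpawnPlayer creates a BP_TrainPawn at the Spawn component's transform and has player controller 0 possess it.
; DisplayStationUI creates the supplied widget class, records the given station on BP_PlayerManager, then adds the widget to the viewport.
; The construction script applies the configurable mesh and world rotation to the static mesh component.
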(event `SpawnPlayer`
  (bind _returnvalue (`|SpawnActorFromClass` "/Game/Blueprints/Gameplay/Player/BP_TrainPawn.BP_TrainPawn_C" (`SceneComponent.K2_GetComponentToWorld` (`self.Spawn`)) "Undefined" "OverrideRootScale" null null))
  (`KismetSystemLibrary.PrintString` "Spawned")
  (`Controller.Possess` (`GameplayStatics.GetPlayerController` 0) _returnvalue))

(event `self.ReceiveBeginPlay`)

(event `DisplayStationUI`
  (params (WdigetClass :type "UserWidget Class Reference") (Station :type "Station Object Reference"))
  (bind _returnvalue (`|CreateWidget` WdigetClass))
  (bind _returnvalue_2 (`GameplayStatics.GetActorOfClass` "/Game/Blueprints/Gameplay/Managers/BP_PlayerManager.BP_PlayerManager_C"))
  (set `/Game/Blueprints/Gameplay/Managers/BP_PlayerManager.Station` Station _returnvalue_2)
  (`UserWidget.AddToViewport` _returnvalue 0))

(fn `UserConstructionScript`
  (bind _staticmesh (`self.StaticMesh`))
  (`StaticMeshComponent.SetStaticMesh` _staticmesh (`self.Mesh`))
  (`SceneComponent.K2_SetWorldRotation` _staticmesh (`self.MeshRotation`) false false))