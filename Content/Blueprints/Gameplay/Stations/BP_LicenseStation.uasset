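; BP_LicenseStation is a station Blueprint that serves as the License Station stop for the train.
; When the train stops, it prints a debug message and has its BP_StationContent child actor display the station's widget UI.
; On BeginPlay, if flagged as a spawn point, it has that same child actor spawn the player.
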(event `self.OnTrainStopped`
  (`KismetSystemLibrary.PrintString` "Tren estacionado en License Station")
  (bind _asbp_station_content (cast `/Game/Blueprints/Gameplay/Stations/BP_StationContent` (`ChildActorComponent.ChildActor` (`self.StationContent`))))
  (`/Game/Blueprints/Gameplay/Stations/BP_StationContent.DisplayStationUI` _asbp_station_content (`self.StationWidget`) self))

(event `self.ReceiveBeginPlay`
  (if (`self.IsSpawnPoint`)
    (bind _asbp_station_content (cast `/Game/Blueprints/Gameplay/Stations/BP_StationContent` (`ChildActorComponent.ChildActor` (`self.StationContent`))))
    (`/Game/Blueprints/Gameplay/Stations/BP_StationContent.SpawnPlayer` _asbp_station_content)))

(fn `UserConstructionScript`)